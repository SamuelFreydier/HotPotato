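; Blueprint function library with a helper that finds the actor of a given class nearest to a target location.
; FindNearestActorOfClass gathers all actors of the class, then runs a linear search comparing each actor's distance to the target against a local running minimum.
; It returns the nearest actor along with its distance.
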(fn `FindNearestActorOfClass`
  (params (Class :type "Actor Class Reference") (TargetLocation :type "Vector Structure"))
  (returns (NearestActor :type "Actor Object Reference") (NearestDistance :type "Float (double-precision)"))
  (locals (Loc_NearestDistance :type "Float (double-precision)") (Loc_NearestActor :type "Actor Object Reference"))
  (bind _outactors (`GameplayStatics.GetAllActorsOfClass` null Class))
  (for _array_element _outactors
    (bind _returnvalue (`KismetMathLibrary.Vector_Distance` (`Actor.K2_GetActorLocation` _array_element) (`local.TargetLocation`)))
    (if (< _returnvalue (`local.Loc_NearestDistance`))
      (set `local.Loc_NearestDistance` _returnvalue)
      (set `local.Loc_NearestActor` _array_element)))
  (return (`local.Loc_NearestActor`) (`local.Loc_NearestDistance`)))