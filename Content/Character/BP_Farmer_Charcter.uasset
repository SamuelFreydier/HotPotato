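; Player farmer character Blueprint with Enhanced Input movement, look and pick-up interaction.
; It adds its input mapping context on BeginPlay and moves relative to the controller's rotation.
; Pick-up stops at the first overlapping actor implementing Interact_Interface and sends it InteractMessage.
; It then plays the interact animation directly on the mesh, restoring Animation Blueprint mode after a fixed delay.
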(event `self.ReceiveBeginPlay`
  (bind _asplayer_controller (cast `PlayerController` (`self.GetController`)))
  (bind _returnvalue (pcsubsystem `EnhancedInputLocalPlayerSubsystem` _asplayer_controller))
  (`/Engine/EditorBlueprintResources/StandardMacros.IsValid` _returnvalue
    (:`Is Valid`
      (`EnhancedInputSubsystemInterface.AddMappingContext` _returnvalue "/Game/Character/Input/IAM_Character.IAM_Character" 0 (struct)))))

(event `EnhancedInput|/Game/Character/Input/IA_Look`
  (params (ActionValue :type "Vector2D Structure") (ElapsedSeconds :type "Float (double-precision)") (TriggeredSeconds :type "Float (double-precision)") (InputAction :type "InputAction Object Reference" :default "/Game/Character/Input/IA_Look.IA_Look"))
  ;[1 1 1] Camera controls
  (:`Triggered`
    (`self.AddControllerYawInput` ActionValue_X)
    (`self.AddControllerPitchInput` ActionValue_Y)))

(event `EnhancedInput|/Game/Character/Input/IA_CharacterMovement`
  (params (ActionValue :type "Vector2D Structure") (ElapsedSeconds :type "Float (double-precision)") (TriggeredSeconds :type "Float (double-precision)") (InputAction :type "InputAction Object Reference" :default "/Game/Character/Input/IA_CharacterMovement.IA_CharacterMovement"))
  (bind (_returnvalue_roll _returnvalue_pitch _returnvalue_yaw) (`KismetMathLibrary.BreakRotator` (`self.GetControlRotation`)))
  (bind (_returnvalue_roll_2 _returnvalue_pitch_2 _returnvalue_yaw_2) (`KismetMathLibrary.BreakRotator` (`self.GetControlRotation`)))
  ;[1 1 1] Movement
  (:`Triggered`
    (`self.AddMovementInput` (`KismetMathLibrary.GetRightVector` (`KismetMathLibrary.MakeRotator` _returnvalue_roll 0.0 _returnvalue_yaw)) ActionValue_X)
    (`self.AddMovementInput` (`KismetMathLibrary.GetForwardVector` (`KismetMathLibrary.MakeRotator` 0.0 0.0 _returnvalue_yaw_2)) ActionValue_Y)))

(event `EnhancedInput|/Game/Character/Input/IA_PickUp`
  (params (ActionValue :type Boolean) (ElapsedSeconds :type "Float (double-precision)") (TriggeredSeconds :type "Float (double-precision)") (InputAction :type "InputAction Object Reference" :default "/Game/Character/Input/IA_PickUp.IA_PickUp"))
  ;[1 1 1] Interaction
  (:`Started`
    (for _array_element (`self.GetOverlappingActors` "/Script/Engine.Actor")
      (if (`KismetSystemLibrary.DoesImplementInterface` _array_element "/Game/Framework/Interact_Interface.Interact_Interface_C")
        (`|ExecutionSequence`
          (:`then_0`
            (break))
          (:`then_1`
            (message `/Game/Framework/Interact_Interface.Interact` _array_element)
            (`SkeletalMeshComponent.PlayAnimation` (`self.Mesh`) "/Game/Character/Farmer/Animation/Farmer_Anim_CharacterArmature_Interact.Farmer_Anim_CharacterArmature_Interact" false)
            (`KismetSystemLibrary.Delay` 1.2)
            (`SkeletalMeshComponent.SetAnimationMode` (`self.Mesh`) "AnimationBlueprint")))))))

(fn `UserConstructionScript`)