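; BP_PlayerCharacter3 is a player character that receives movement and interaction through custom events rather than handling input itself.
; SendTest turns vertical and horizontal values into movement along fixed world X and Y axes.
; SendP2Interaction plays a one-shot mesh animation, restores Animation Blueprint mode after a delay, then sends InteractMessage to the first overlapping actor implementing the interface.
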(event `self.ReceiveTick`
  (params (DeltaSeconds :type "Float (single-precision)")))

(event `/Game/Character/BPI_CoopControl.Send_Test`
  (params (ver :type "Float (double-precision)") (hor :type "Float (double-precision)"))
  ;[1 1 1] Movement
  (`self.AddMovementInput` (0.0 1.0 0.0) hor)
  (`self.AddMovementInput` (1.0 0.0 0.0) ver))

(event `/Game/Character/BPI_CoopControl.Send_P2_Interaction`
  ;[1 1 1] Interaction
  (`SkeletalMeshComponent.PlayAnimation` (`self.Mesh`) null false)
  (`KismetSystemLibrary.Delay` 1.2)
  (`SkeletalMeshComponent.SetAnimationMode` (`self.Mesh`) "AnimationBlueprint")
  (for _array_element (`self.GetOverlappingActors` "/Script/Engine.Actor")
    (if (`KismetSystemLibrary.DoesImplementInterface` _array_element)
      (`|ExecutionSequence`
        (:`then_0`
          (break))
        (:`then_1`
          (message `/Game/Framework/Interact_Interface.Interact` _array_element null))))))

(fn `UserConstructionScript`)