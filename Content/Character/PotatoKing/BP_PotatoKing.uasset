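; BP_PotatoKing is the Potato King actor that players interact with to hand over potatoes.
; On begin play it runs inherited setup and initializes base gluttony and score offset.
; Interacting calls GivePotatoes on the player character and plays a random sound from its list at the King's location.
; Tick watches the Terminated flag, then shows the mouse cursor and opens the main menu level.
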(event `self.ReceiveBeginPlay`
  (`self.PotatoBeginPlay`)
  (`self.Init` 5))

(event `/Game/Framework/Interact_Interface.Interact`
  (params (Player :type "Actor Object Reference"))
  (bind _ashot_potato_character (cast `HotPotatoCharacter` Player))
  (`HotPotatoCharacter.GivePotatoes` _ashot_potato_character self)
  (bind _randomelement (`self.GetRandomSoundFromList` (`self.SoundList`)))
  (`GameplayStatics.PlaySoundAtLocation` _randomelement (`self.K2_GetActorLocation`) (struct) 0.6 1.0 0.0 null null null null))

(event `self.ReceiveTick`
  (params (DeltaSeconds :type "Float (single-precision)"))
  (if (`self.bTerminated`)
    (set `PlayerController.bShowMouseCursor` true (`GameplayStatics.GetPlayerController` 0))
    (`GameplayStatics.OpenLevelBySoftObjectPtr` "/Game/Menus/MainMenuMap.MainMenuMap")))

(fn `GetRandomSoundFromList`
  (params (Array :type "Array of SoundWave Object Reference"))
  (returns (RandomElement :type "SoundWave Object Reference"))
  (return (`|GetArrayItem` Array (`KismetMathLibrary.RandomInteger` (`KismetArrayLibrary.Array_Length` Array)))))

(fn `UserConstructionScript`)