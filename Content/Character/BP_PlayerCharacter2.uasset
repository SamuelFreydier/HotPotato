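; Player-one character for two-player play that also relays player-two input to BP_PlayerCharacter3 actors found at BeginPlay.
; P1 axes drive movement relative to control rotation, while P2 movement and action inputs are forwarded through calls on those actors.
; P1's action plays a pick animation, waits, restores the animation Blueprint, then sends InteractMessage to the first overlapping actor implementing the interface.
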(event `self.ReceiveBeginPlay`
  (bind _outactors (`GameplayStatics.GetAllActorsOfClass` "/Game/Character/BP_PlayerCharacter3.BP_PlayerCharacter3_C"))
  (set `self.Out Actors` _outactors))

(event `InputAxis|P1_Horizontal`
  (params (AxisValue :type "Float (single-precision)"))
  (bind (_returnvalue_roll _returnvalue_pitch _returnvalue_yaw) (`KismetMathLibrary.BreakRotator` (`self.GetControlRotation`)))
  ;[1 1 1] Movement
  (`self.AddMovementInput` (`KismetMathLibrary.GetRightVector` (`KismetMathLibrary.MakeRotator` _returnvalue_roll 0.0 _returnvalue_yaw)) AxisValue))

(event `InputAxis|P1_Vertical`
  (params (AxisValue :type "Float (single-precision)"))
  (bind (_returnvalue_roll _returnvalue_pitch _returnvalue_yaw) (`KismetMathLibrary.BreakRotator` (`self.GetControlRotation`)))
  ;[1 1 1] Movement
  (`self.AddMovementInput` (`KismetMathLibrary.GetForwardVector` (`KismetMathLibrary.MakeRotator` 0.0 0.0 _returnvalue_yaw)) AxisValue))

(event `InputAxis|P2_Vertical`
  (params (AxisValue :type "Float (single-precision)"))
  (`/Game/Character/BP_PlayerCharacter3.Send_P2_MovementVertical` (`self.Out Actors`) AxisValue))

(event `InputAxis|P2_Horizontal`
  (params (AxisValue :type "Float (single-precision)"))
  (`self.Send_P2_MovementHorizontal` (`self.Out Actors`) AxisValue))

(event `InputAction|P2_Action`
  (params (Key :type "Key Structure"))
  (:`Pressed`
    (`self.Send_P2_Interaction` (`self.Out Actors`))))

(event `InputAction|P1_Action`
  (params (Key :type "Key Structure"))
  ;[1 1 1] Interaction
  (:`Pressed`
    (`SkeletalMeshComponent.PlayAnimation` (`self.Mesh`) "/Game/Character/Animations/Character_Pick.Character_Pick" false)
    (`KismetSystemLibrary.Delay` 1.2)
    (`SkeletalMeshComponent.SetAnimationMode` (`self.Mesh`) "AnimationBlueprint")
    (for _array_element (`self.GetOverlappingActors` "/Script/Engine.Actor")
      (if (`KismetSystemLibrary.DoesImplementInterface` _array_element)
        (`|ExecutionSequence`
          (:`then_0`
            (break))
          (:`then_1`
            (message `/Game/Framework/Interact_Interface.Interact` _array_element)))))))

(fn `UserConstructionScript`)