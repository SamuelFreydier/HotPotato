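; BP_P01 is a player character Blueprint, apparently for player one, with most of its logic disconnected.
; Its P1 axis events are empty, and the mapping context setup, possession, look, movement, pick animation and interface-based overlap interaction chains never run.
; The GrowPlant event plays a timeline that multiplies the target's current relative scale by the track value each update, then prints a debug string; its only call here is disconnected.
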(event `self.ReceiveBeginPlay`)

(event `EnhancedInput|/Game/Character/Input/IA_Look`
  (params (ActionValue :type "Vector2D Structure") (ElapsedSeconds :type "Float (double-precision)") (TriggeredSeconds :type "Float (double-precision)") (InputAction :type "InputAction Object Reference" :default "/Game/Character/Input/IA_Look.IA_Look"))
  ;[1 1 1] Camera controls
)

(event `EnhancedInput|/Game/Character/Input/IA_CharacterMovement`
  (params (ActionValue :type "Vector2D Structure") (ElapsedSeconds :type "Float (double-precision)") (TriggeredSeconds :type "Float (double-precision)") (InputAction :type "InputAction Object Reference" :default "/Game/Character/Input/IA_CharacterMovement.IA_CharacterMovement")))

(event `InputAxis|P1_Vertical`
  (params (AxisValue :type "Float (single-precision)"))
  ;[1 1 1] Movement
)

(event `InputAxis|P1_Horizontal`
  (params (AxisValue :type "Float (single-precision)"))
  ;[1 1 1] Movement
)

(event `EnhancedInput|/Game/Character/Input/IA_PickUp`
  (params (ActionValue :type Boolean) (ElapsedSeconds :type "Float (double-precision)") (TriggeredSeconds :type "Float (double-precision)") (InputAction :type "InputAction Object Reference" :default "/Game/Character/Input/IA_PickUp.IA_PickUp")))

(event `InputAction|P1_Action`
  (params (Key :type "Key Structure"))
  ;[1 1 1] Interaction
)

(event `GrowPlant`
  (params (Target :type "SceneComponent Object Reference"))
  (bind (_direction _newtrack_0) (`Timeline|Timeline` :!via `PlayFromStart`)
    (:`Update`
      (`SceneComponent.SetRelativeScale3D` Target (* (`SceneComponent.RelativeScale3D` Target) _newtrack_0)))
    (:`Finished`
      (`KismetSystemLibrary.PrintString` "Hello"))))

(fn `UserConstructionScript`)