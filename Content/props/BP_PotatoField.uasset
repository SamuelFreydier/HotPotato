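; Potato field prop that endlessly cycles through growing, a timed harvest window and rotting.
; A delay-driven loop from BeginPlay grows six BP_PotatoPlant_1 child actors, shows a collectible potato, then removes the plants and briefly shows a rotten potato if uncollected.
; Interact during the window hides the potato and flags it collected, without granting any item here.
; Tick continuously spins the potato, with the rotten one following its rotation.
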(event `self.ReceiveBeginPlay`
  (`self.PlantsStonks` :!label _label)
  (`KismetSystemLibrary.Delay` 8.0)
  (set `self.CanBeCollected` true)
  (set `self.HasBeenCollected` false)
  (`SceneComponent.SetVisibility` (`self.Potato`) true false)
  (`KismetSystemLibrary.Delay` 12.0)
  (`SceneComponent.SetVisibility` (`self.Potato`) false false)
  (if (not (`self.HasBeenCollected`))
    (`SceneComponent.SetVisibility` (`self.Rotten_potato`) true false))
  (`self.PlantsNotStonks`)
  (set `self.CanBeCollected` false)
  (`KismetSystemLibrary.Delay` 5.0)
  (`SceneComponent.SetVisibility` (`self.Rotten_potato`) false false)
  (goto _label))

(event `/Game/Framework/Interact_Interface.Interact`
  (if (`self.CanBeCollected`)
    (set `self.HasBeenCollected` true)
    (`SceneComponent.SetVisibility` (`self.Potato`) false false)
    (set `self.CanBeCollected` false)))

(event `self.ReceiveTick`
  (params (DeltaSeconds :type "Float (single-precision)"))
  (bind _potato (`self.Potato`))
  (bind _returnvalue (`KismetMathLibrary.Conv_VectorToRotator` (`KismetMathLibrary.GreaterGreater_VectorRotator` (`KismetMathLibrary.Conv_RotatorToVector` (`SceneComponent.RelativeRotation` _potato)) (struct :`Yaw` 2.0))))
  (`SceneComponent.K2_SetRelativeRotation` _potato _returnvalue false false)
  (`SceneComponent.K2_SetRelativeRotation` (`self.Rotten_potato`) _returnvalue false false))

(event `PlantsStonks`
  (bind _asbp_potato_plant_1 (cast `/Game/props/BP_PotatoPlant_1` (`ChildActorComponent.ChildActor` (`self.Plant1`))))
  (bind _asbp_potato_plant_1_2 (cast `/Game/props/BP_PotatoPlant_1` (`ChildActorComponent.ChildActor` (`self.Plant2`))))
  (bind _asbp_potato_plant_1_3 (cast `/Game/props/BP_PotatoPlant_1` (`ChildActorComponent.ChildActor` (`self.Plant3`))))
  (bind _asbp_potato_plant_1_4 (cast `/Game/props/BP_PotatoPlant_1` (`ChildActorComponent.ChildActor` (`self.Plant4`))))
  (bind _asbp_potato_plant_1_5 (cast `/Game/props/BP_PotatoPlant_1` (`ChildActorComponent.ChildActor` (`self.Plant5`))))
  (bind _asbp_potato_plant_1_6 (cast `/Game/props/BP_PotatoPlant_1` (`ChildActorComponent.ChildActor` (`self.Plant6`))))
  (`/Game/props/BP_PotatoPlant_1.GrowPlant` _asbp_potato_plant_1)
  (`/Game/props/BP_PotatoPlant_1.GrowPlant` _asbp_potato_plant_1_2)
  (`/Game/props/BP_PotatoPlant_1.GrowPlant` _asbp_potato_plant_1_3)
  (`/Game/props/BP_PotatoPlant_1.GrowPlant` _asbp_potato_plant_1_4)
  (`/Game/props/BP_PotatoPlant_1.GrowPlant` _asbp_potato_plant_1_5)
  (`/Game/props/BP_PotatoPlant_1.GrowPlant` _asbp_potato_plant_1_6))

(event `PlantsNotStonks`
  (bind _asbp_potato_plant_1 (cast `/Game/props/BP_PotatoPlant_1` (`ChildActorComponent.ChildActor` (`self.Plant1`))))
  (bind _asbp_potato_plant_1_2 (cast `/Game/props/BP_PotatoPlant_1` (`ChildActorComponent.ChildActor` (`self.Plant2`))))
  (bind _asbp_potato_plant_1_3 (cast `/Game/props/BP_PotatoPlant_1` (`ChildActorComponent.ChildActor` (`self.Plant3`))))
  (bind _asbp_potato_plant_1_4 (cast `/Game/props/BP_PotatoPlant_1` (`ChildActorComponent.ChildActor` (`self.Plant4`))))
  (bind _asbp_potato_plant_1_5 (cast `/Game/props/BP_PotatoPlant_1` (`ChildActorComponent.ChildActor` (`self.Plant5`))))
  (bind _asbp_potato_plant_1_6 (cast `/Game/props/BP_PotatoPlant_1` (`ChildActorComponent.ChildActor` (`self.Plant6`))))
  (`/Game/props/BP_PotatoPlant_1.PlantDisapear` _asbp_potato_plant_1_6)
  (`/Game/props/BP_PotatoPlant_1.PlantDisapear` _asbp_potato_plant_1_5)
  (`/Game/props/BP_PotatoPlant_1.PlantDisapear` _asbp_potato_plant_1_4)
  (`/Game/props/BP_PotatoPlant_1.PlantDisapear` _asbp_potato_plant_1_3)
  (`/Game/props/BP_PotatoPlant_1.PlantDisapear` _asbp_potato_plant_1_2)
  (`/Game/props/BP_PotatoPlant_1.PlantDisapear` _asbp_potato_plant_1))

(fn `UserConstructionScript`)