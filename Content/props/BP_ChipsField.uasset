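; BP_ChipsField is a potato field prop that cyclically produces chips the player can gather.
; A looping BeginPlay delay chain grows six child-actor plants, shows collectible chips, then removes the plants and briefly shows rotten chips if none were collected.
; Interact during the collectible window gives player 0's HotPotatoCharacter one CHIPS and hides the mesh.
; Tick rotates the fresh chips mesh and sets the rotten mesh's rotation from it.
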(event `self.ReceiveBeginPlay`
  (`self.PlantsStonks` :!label _label)
  (`KismetSystemLibrary.Delay` 10.0)
  (set `self.CanBeCollected` true)
  (set `self.HasBeenCollected` false)
  (`SceneComponent.SetVisibility` (`self.SM_Chips`) true false)
  (`KismetSystemLibrary.Delay` 10.0)
  (`SceneComponent.SetVisibility` (`self.SM_Chips`) false false)
  (if (not (`self.HasBeenCollected`))
    (`SceneComponent.SetVisibility` (`self.SM_ChipsPourrie`) true false))
  (`self.PlantsNotStonks`)
  (set `self.CanBeCollected` false)
  (`KismetSystemLibrary.Delay` 5.0)
  (`SceneComponent.SetVisibility` (`self.SM_ChipsPourrie`) false false)
  (goto _label))

(event `/Game/Framework/Interact_Interface.Interact`
  (params (Player :type "Actor Object Reference"))
  (if (`self.CanBeCollected`)
    (set `self.HasBeenCollected` true)
    (bind _ashot_potato_character (cast `HotPotatoCharacter` (`GameplayStatics.GetPlayerCharacter` 0)))
    (`HotPotatoCharacter.GatherPotato` _ashot_potato_character "CHIPS" 1)
    (`SceneComponent.SetVisibility` (`self.SM_Chips`) false false)
    (set `self.CanBeCollected` false)))

(event `self.ReceiveTick`
  (params (DeltaSeconds :type "Float (single-precision)"))
  (bind _returnvalue (`KismetMathLibrary.Conv_VectorToRotator` (`KismetMathLibrary.GreaterGreater_VectorRotator` (`KismetMathLibrary.Conv_RotatorToVector` (`SceneComponent.RelativeRotation` (`self.SM_Chips`))) (struct :`Yaw` 2.0))))
  (`SceneComponent.K2_SetRelativeRotation` (`self.SM_Chips`) _returnvalue false false)
  (`SceneComponent.K2_SetRelativeRotation` (`self.SM_ChipsPourrie`) _returnvalue false false))

(event `PlantsStonks`
  (bind _asbp_potato_plant_3 (cast `/Game/Props/potatoplant/BP_Potato_Plant3` (`ChildActorComponent.ChildActor` (`self.Plant1`))))
  (bind _asbp_potato_plant_3_2 (cast `/Game/Props/potatoplant/BP_Potato_Plant3` (`ChildActorComponent.ChildActor` (`self.Plant2`))))
  (bind _asbp_potato_plant_3_3 (cast `/Game/Props/potatoplant/BP_Potato_Plant3` (`ChildActorComponent.ChildActor` (`self.Plant3`))))
  (bind _asbp_potato_plant_3_4 (cast `/Game/Props/potatoplant/BP_Potato_Plant3` (`ChildActorComponent.ChildActor` (`self.Plant4`))))
  (bind _asbp_potato_plant_3_5 (cast `/Game/Props/potatoplant/BP_Potato_Plant3` (`ChildActorComponent.ChildActor` (`self.Plant5`))))
  (bind _asbp_potato_plant_3_6 (cast `/Game/Props/potatoplant/BP_Potato_Plant3` (`ChildActorComponent.ChildActor` (`self.Plant6`))))
  (`/Game/Props/potatoplant/BP_Potato_Plant3.GrowPlant` _asbp_potato_plant_3_6)
  (`/Game/Props/potatoplant/BP_Potato_Plant3.GrowPlant` _asbp_potato_plant_3_5)
  (`/Game/Props/potatoplant/BP_Potato_Plant3.GrowPlant` _asbp_potato_plant_3_4)
  (`/Game/Props/potatoplant/BP_Potato_Plant3.GrowPlant` _asbp_potato_plant_3_3)
  (`/Game/Props/potatoplant/BP_Potato_Plant3.GrowPlant` _asbp_potato_plant_3_2)
  (`/Game/Props/potatoplant/BP_Potato_Plant3.GrowPlant` _asbp_potato_plant_3))

(event `PlantsNotStonks`
  (bind _asbp_potato_plant_3 (cast `/Game/Props/potatoplant/BP_Potato_Plant3` (`ChildActorComponent.ChildActor` (`self.Plant1`))))
  (bind _asbp_potato_plant_3_2 (cast `/Game/Props/potatoplant/BP_Potato_Plant3` (`ChildActorComponent.ChildActor` (`self.Plant2`))))
  (bind _asbp_potato_plant_3_3 (cast `/Game/Props/potatoplant/BP_Potato_Plant3` (`ChildActorComponent.ChildActor` (`self.Plant3`))))
  (bind _asbp_potato_plant_3_4 (cast `/Game/Props/potatoplant/BP_Potato_Plant3` (`ChildActorComponent.ChildActor` (`self.Plant4`))))
  (bind _asbp_potato_plant_3_5 (cast `/Game/Props/potatoplant/BP_Potato_Plant3` (`ChildActorComponent.ChildActor` (`self.Plant5`))))
  (bind _asbp_potato_plant_3_6 (cast `/Game/Props/potatoplant/BP_Potato_Plant3` (`ChildActorComponent.ChildActor` (`self.Plant6`))))
  (`/Game/Props/potatoplant/BP_Potato_Plant3.PlantDisapear` _asbp_potato_plant_3_6)
  (`/Game/Props/potatoplant/BP_Potato_Plant3.PlantDisapear` _asbp_potato_plant_3_5)
  (`/Game/Props/potatoplant/BP_Potato_Plant3.PlantDisapear` _asbp_potato_plant_3_4)
  (`/Game/Props/potatoplant/BP_Potato_Plant3.PlantDisapear` _asbp_potato_plant_3_3)
  (`/Game/Props/potatoplant/BP_Potato_Plant3.PlantDisapear` _asbp_potato_plant_3)
  (`/Game/Props/potatoplant/BP_Potato_Plant3.PlantDisapear` _asbp_potato_plant_3_2))

(fn `UserConstructionScript`)