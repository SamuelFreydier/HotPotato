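; Farm field prop that repeatedly grows a poutine for the player to harvest.
; A delay-driven BeginPlay loop grows six child-actor potato plants, reveals a collectible poutine briefly, then removes the plants, showing rotten poutine if uncollected.
; Interact during that window grants one POUTINE through the player's GatherPotato and hides it.
; Tick spins both poutine components, deriving the rotten one's rotation from the fresh one's.
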(event `self.ReceiveBeginPlay`
  (bind _poutine (`self.Poutine`))
  (bind _rottenpoutine (`self.RottenPoutine`))
  (`self.PlantsStonks` :!label _label)
  (`KismetSystemLibrary.Delay` 14.0)
  (set `self.CanBeCollected` true)
  (set `self.HasBeenCollected` false)
  (`SceneComponent.SetVisibility` _poutine true false)
  (`KismetSystemLibrary.Delay` 6.0)
  (`SceneComponent.SetVisibility` _poutine false false)
  (if (not (`self.HasBeenCollected`))
    (`SceneComponent.SetVisibility` _rottenpoutine true false))
  (`self.PlantsNotStonks`)
  (set `self.CanBeCollected` false)
  (`KismetSystemLibrary.Delay` 5.0)
  (`SceneComponent.SetVisibility` _rottenpoutine false false)
  (goto _label))

(event `/Game/Framework/Interact_Interface.Interact`
  (params (Player :type "Actor Object Reference"))
  (if (`self.CanBeCollected`)
    (set `self.HasBeenCollected` true)
    (bind _ashot_potato_character (cast `HotPotatoCharacter` (`GameplayStatics.GetPlayerCharacter` 0)))
    (`HotPotatoCharacter.GatherPotato` _ashot_potato_character "POUTINE" 1)
    (`SceneComponent.SetVisibility` (`self.Poutine`) false false)
    (set `self.CanBeCollected` false)))

(event `self.ReceiveTick`
  (params (DeltaSeconds :type "Float (single-precision)"))
  (bind _poutine (`self.Poutine`))
  (bind _returnvalue (`KismetMathLibrary.Conv_VectorToRotator` (`KismetMathLibrary.GreaterGreater_VectorRotator` (`KismetMathLibrary.Conv_RotatorToVector` (`SceneComponent.RelativeRotation` _poutine)) (struct :`Yaw` 2.0))))
  (`SceneComponent.K2_SetRelativeRotation` _poutine _returnvalue false false)
  (`SceneComponent.K2_SetRelativeRotation` (`self.RottenPoutine`) _returnvalue false false))

(event `PlantsStonks`
  (bind _asbp_potato_plant_4 (cast `/Game/Props/potatoplant/BP_Potato_Plant4` (`ChildActorComponent.ChildActor` (`self.Plant1`))))
  (bind _asbp_potato_plant_4_2 (cast `/Game/Props/potatoplant/BP_Potato_Plant4` (`ChildActorComponent.ChildActor` (`self.Plant2`))))
  (bind _asbp_potato_plant_4_3 (cast `/Game/Props/potatoplant/BP_Potato_Plant4` (`ChildActorComponent.ChildActor` (`self.Plant3`))))
  (bind _asbp_potato_plant_4_4 (cast `/Game/Props/potatoplant/BP_Potato_Plant4` (`ChildActorComponent.ChildActor` (`self.Plant4`))))
  (bind _asbp_potato_plant_4_5 (cast `/Game/Props/potatoplant/BP_Potato_Plant4` (`ChildActorComponent.ChildActor` (`self.Plant5`))))
  (bind _asbp_potato_plant_4_6 (cast `/Game/Props/potatoplant/BP_Potato_Plant4` (`ChildActorComponent.ChildActor` (`self.Plant6`))))
  (`/Game/Props/potatoplant/BP_Potato_Plant4.GrowPlant` _asbp_potato_plant_4)
  (`/Game/Props/potatoplant/BP_Potato_Plant4.GrowPlant` _asbp_potato_plant_4_6)
  (`/Game/Props/potatoplant/BP_Potato_Plant4.GrowPlant` _asbp_potato_plant_4_5)
  (`/Game/Props/potatoplant/BP_Potato_Plant4.GrowPlant` _asbp_potato_plant_4_2)
  (`/Game/Props/potatoplant/BP_Potato_Plant4.GrowPlant` _asbp_potato_plant_4_3)
  (`/Game/Props/potatoplant/BP_Potato_Plant4.GrowPlant` _asbp_potato_plant_4_4))

(event `PlantsNotStonks`
  (bind _asbp_potato_plant_4 (cast `/Game/Props/potatoplant/BP_Potato_Plant4` (`ChildActorComponent.ChildActor` (`self.Plant1`))))
  (bind _asbp_potato_plant_4_2 (cast `/Game/Props/potatoplant/BP_Potato_Plant4` (`ChildActorComponent.ChildActor` (`self.Plant2`))))
  (bind _asbp_potato_plant_4_3 (cast `/Game/Props/potatoplant/BP_Potato_Plant4` (`ChildActorComponent.ChildActor` (`self.Plant3`))))
  (bind _asbp_potato_plant_4_4 (cast `/Game/Props/potatoplant/BP_Potato_Plant4` (`ChildActorComponent.ChildActor` (`self.Plant4`))))
  (bind _asbp_potato_plant_4_5 (cast `/Game/Props/potatoplant/BP_Potato_Plant4` (`ChildActorComponent.ChildActor` (`self.Plant5`))))
  (bind _asbp_potato_plant_4_6 (cast `/Game/Props/potatoplant/BP_Potato_Plant4` (`ChildActorComponent.ChildActor` (`self.Plant6`))))
  (`/Game/Props/potatoplant/BP_Potato_Plant4.PlantDisapear` _asbp_potato_plant_4_6)
  (`/Game/Props/potatoplant/BP_Potato_Plant4.PlantDisapear` _asbp_potato_plant_4)
  (`/Game/Props/potatoplant/BP_Potato_Plant4.PlantDisapear` _asbp_potato_plant_4_2)
  (`/Game/Props/potatoplant/BP_Potato_Plant4.PlantDisapear` _asbp_potato_plant_4_3)
  (`/Game/Props/potatoplant/BP_Potato_Plant4.PlantDisapear` _asbp_potato_plant_4_4)
  (`/Game/Props/potatoplant/BP_Potato_Plant4.PlantDisapear` _asbp_potato_plant_4_5))

(fn `UserConstructionScript`)