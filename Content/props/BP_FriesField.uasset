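; Fries field prop that repeatedly grows fries, which a player can harvest through Interact to gather one FRIES potato.
; BeginPlay runs an endless Delay-driven cycle: wait, show fries as collectable, then hide them and, if uncollected, briefly show an uncollectable rotten mesh.
; Interact grants the potato, hides the fries and flags them collected, so the cycle skips the rotten stage.
; Tick spins both meshes by a fixed per-frame step, independent of delta time.
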(event `self.ReceiveBeginPlay`
  (bind _sm_friesrotten (`self.SM_FriesRotten`))
  (`KismetSystemLibrary.Delay` 5.0 :!label _label)
  (set `self.CanBeCollected` true)
  (set `self.HasBeenCollected` false)
  (`SceneComponent.SetVisibility` (`self.SM_Fries`) true false)
  (`KismetSystemLibrary.Delay` 5.0)
  (`SceneComponent.SetVisibility` (`self.SM_Fries`) false false)
  (if (`self.HasBeenCollected`)
    (goto _label)
    (else
      (`SceneComponent.SetVisibility` _sm_friesrotten true false)
      (set `self.CanBeCollected` false)
      (`KismetSystemLibrary.Delay` 4.0)
      (`SceneComponent.SetVisibility` _sm_friesrotten false false)
      (goto _label))))

(event `/Game/Framework/Interact_Interface.Interact`
  (params (Player :type "Actor Object Reference"))
  (if (`self.CanBeCollected`)
    (set `self.HasBeenCollected` true)
    (bind _ashot_potato_character (cast `HotPotatoCharacter` Player))
    (`HotPotatoCharacter.GatherPotato` _ashot_potato_character "FRIES" 1)
    (`SceneComponent.SetVisibility` (`self.SM_Fries`) false false)
    (set `self.CanBeCollected` false)))

(event `self.ReceiveTick`
  (params (DeltaSeconds :type "Float (single-precision)"))
  (bind _sm_fries (`self.SM_Fries`))
  (bind _returnvalue (`KismetMathLibrary.Conv_VectorToRotator` (`KismetMathLibrary.GreaterGreater_VectorRotator` (`KismetMathLibrary.Conv_RotatorToVector` (`SceneComponent.RelativeRotation` _sm_fries)) (struct :`Yaw` 2.0))))
  (`SceneComponent.K2_SetRelativeRotation` _sm_fries _returnvalue false false)
  (`SceneComponent.K2_SetRelativeRotation` (`self.SM_FriesRotten`) _returnvalue false false))

(fn `UserConstructionScript`)