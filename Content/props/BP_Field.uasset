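; BP_Field is a farm field prop that cycles a potato through growing, ripe and rotten stages.
; A looping Delay chain from BeginPlay toggles the Potato and RottenPotato visibility and sets the collection flags.
; Interact hides the potato and flags it collected while collectable, without granting an item.
; If collected, the cycle restarts after the ripe window; otherwise the rotten potato shows briefly and blocks collection first.
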(event `self.ReceiveBeginPlay`
  (`KismetSystemLibrary.Delay` 5.0 :!label _label)
  (set `self.CanBeCollected` true)
  (set `self.HasBeenCollected` false)
  (`SceneComponent.SetVisibility` (`self.Potato`) true false)
  (`KismetSystemLibrary.Delay` 5.0)
  (`SceneComponent.SetVisibility` (`self.Potato`) false false)
  (if (`self.HasBeenCollected`)
    (`KismetSystemLibrary.PrintString` "hasbeencollected")
    (goto _label)
    (else
      (`SceneComponent.SetVisibility` (`self.Rotten_potato`) true false)
      (set `self.CanBeCollected` false)
      (`KismetSystemLibrary.Delay` 4.0)
      (`SceneComponent.SetVisibility` (`self.Rotten_potato`) false false)
      (goto _label))))

(event `/Game/Framework/Interact_Interface.Interact`
  (`KismetSystemLibrary.PrintString` "Hello" true true (struct :`G` 0.66 :`B` 1.0 :`A` 1.0) 10.0)
  (if (`self.CanBeCollected`)
    (set `self.HasBeenCollected` true)
    (`SceneComponent.SetVisibility` (`self.Potato`) false false)))

(fn `UserConstructionScript`)